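; BP_JsonListEntry is a hierarchical list entry that reads and edits fields in a shared JSON document, including issue totals.
; Path-based getters and setters work on the root entry's JSON string, falling back to itself when no root is set.
; Issue-count changes write total_issues at the entry's path and propagate recursively up the Parent chain.
; Optional refreshes go through UtilityAction, deferred to the top of the chain for count updates.
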(fn SetStringFieldValue
  (params (Path :type Text) (Value :type String) (Refresh :type Boolean))
  (bind _rootjson (CallFunction|GetRootJson))
  (bind _returnvalue (CallFunction|SetStringJsonValue (Variables|BP_JsonListEntry_C|GetJsonString _rootjson) (Utilities|String|ToString(Text) Path) Value))
  (Variables|BP_JsonListEntry_C|SetJsonString _rootjson _returnvalue)
  (if Refresh
    (CallFunction|Refresh)))

(fn SetBoolFieldValue
  (params (Path :type Text) (Value :type Boolean) (refresh :type Boolean))
  (bind _rootjson (CallFunction|GetRootJson))
  (bind _returnvalue (CallFunction|SetBoolJsonValue (Variables|BP_JsonListEntry_C|GetJsonString _rootjson) (Utilities|String|ToString(Text) Path) Value))
  (Variables|BP_JsonListEntry_C|SetJsonString _rootjson _returnvalue)
  (if refresh
    (CallFunction|Refresh)))

(fn GetSubJson
  (params (Path :type Text))
  (bind _returnvalue (CallFunction|GetJsonValue (Variables|BP_JsonListEntry_C|GetJsonString (CallFunction|GetRootJson)) (Utilities|String|ToString(Text) Path)))
  (bind (_outjsonobject _returnvalue_2) (Class|JsonBlueprintFunctionLibrary|FromString _returnvalue))
  (return _outjsonobject _returnvalue_2))

(fn SetIntFieldValue
  (params (Path :type Text) (Value :type Integer) (refresh :type Boolean))
  (bind _rootjson (CallFunction|GetRootJson))
  (bind _returnvalue (CallFunction|SetIntJsonValue (Variables|BP_JsonListEntry_C|GetJsonString _rootjson) (Utilities|String|ToString(Text) Path) Value))
  (Variables|BP_JsonListEntry_C|SetJsonString _rootjson _returnvalue)
  (if refresh
    (CallFunction|Refresh)))

(fn Refresh
  (Default|CallRefresh (Variables|Default|GetUtilityAction)))

(fn AddNbIssuesValue
  (params (value :type Integer) (Refresh :type Boolean))
  (bind _jsonpath (Variables|Default|GetJsonPath))
  (if (!= value 0)
    (Variables|Default|SetNbIssues (+ value (Variables|Default|GetNbIssues)))
    (if (Utilities|Text|TextIsEmpty _jsonpath)
      (LocalVariables|Setkey "total_issues")
      (else
        (LocalVariables|Setkey (Utilities|Text|FormatText "{parent}.total_issues" _jsonpath))))
    (CallFunction|SetIntFieldValue (LocalVariables|Getkey) (Variables|Default|GetNbIssues) false)
    (Utilities|IsValid (Variables|Default|GetParent)
      (:Is%20Valid
        (CallFunction|AddNbIssuesValue (Variables|Default|GetParent) value Refresh))
      (:Is%20Not%20Valid
        (if Refresh
          (CallFunction|Refresh))))
    (elif Refresh
      (CallFunction|Refresh))))

(fn GetRootJson
  (bind _rootjson (Variables|Default|GetRootJson))
  (Utilities|IsValid _rootjson
    (:Is%20Valid
      (return _rootjson))
    (:Is%20Not%20Valid
      (return self))))